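; BP_CoreItem is a world item actor that hands itself to the inventory component of actors overlapping its box.
; With AutoPickUp on, it calls FAddItemMessage and destroys itself; otherwise it registers as an overlapping item and pickup target, showing the interaction prompt for the first one.
; End overlap deregisters it and hides the prompt when none remain.
; Construction sets optional mesh physics with physics-only collision.
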(event `self.ReceiveBeginPlay`)

(event `self.Box.OnComponentBeginOverlap`
  (params (OverlappedComponent :type "PrimitiveComponent Object Reference") (OtherActor :type "Actor Object Reference") (OtherComp :type "PrimitiveComponent Object Reference") (OtherBodyIndex :type Integer) (bFromSweep :type Boolean) (SweepResult :type "HitResult Structure (by ref)"))
  (bind _returnvalue (`self.GetComponentByClass` OtherActor "/Game/InventoryComponent/AC_InventoryComponent.AC_InventoryComponent_C"))
  (bind _overlappingitems (`/Game/InventoryComponent/AC_InventoryComponent.OverlappingItems` _returnvalue))
  (if (`KismetSystemLibrary.IsValid` _returnvalue)
    (if (`/Game/InventoryComponent/AC_InventoryComponent.AutoPickUp` _returnvalue)
      ;[1 1 1] Logic for NPC
      (message `/Game/InventoryComponent/BPI_InventoryInterface.F_AddItem` _returnvalue self)
      (`self.K2_DestroyActor`)
      (else
        (`KismetArrayLibrary.Array_Add` _overlappingitems self)
        (set `/Game/InventoryComponent/AC_InventoryComponent.ItemToPickup` self _returnvalue)
        (if (== (`KismetArrayLibrary.Array_Length` _overlappingitems) 1)
          (if true
            (`/Game/InventoryComponent/AC_InventoryComponent.F_SetInterectionVisibility` _returnvalue true)))))))

(event `self.Box.OnComponentEndOverlap`
  (params (OverlappedComponent :type "PrimitiveComponent Object Reference") (OtherActor :type "Actor Object Reference") (OtherComp :type "PrimitiveComponent Object Reference") (OtherBodyIndex :type Integer))
  (bind _returnvalue (`self.GetComponentByClass` OtherActor "/Game/InventoryComponent/AC_InventoryComponent.AC_InventoryComponent_C"))
  (bind _overlappingitems (`/Game/InventoryComponent/AC_InventoryComponent.OverlappingItems` _returnvalue))
  (`/Engine/EditorBlueprintResources/StandardMacros.IsValid` OtherActor
    (:`Is Valid`
      (if (`KismetSystemLibrary.DoesImplementInterface` _returnvalue "/Game/InventoryComponent/BPI_InventoryInterface.BPI_InventoryInterface_C")
        (`KismetArrayLibrary.Array_RemoveItem` _overlappingitems self)
        (if (not (> (`KismetArrayLibrary.Array_Length` _overlappingitems) 0))
          (`/Game/InventoryComponent/AC_InventoryComponent.F_SetInterectionVisibility` _returnvalue false))))))

(fn `UserConstructionScript`
  (bind _staticmesh (`self.StaticMesh`))
  (`PrimitiveComponent.SetSimulatePhysics` _staticmesh (`self.UsePhysics`))
  (`PrimitiveComponent.SetCollisionEnabled` _staticmesh "PhysicsOnly"))